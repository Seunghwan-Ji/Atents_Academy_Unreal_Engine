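; BP_Weapon is a weapon actor that deals damage to actors it overlaps, excluding its instigator.
; Overlap applies its Damage value, crediting the instigator's controller and naming the weapon as damage causer.
; GetStateMontageData looks up montage, play rate and section by state and index from StateMontageMap.
; BeginAttack and EndAttack are empty, so nothing here limits damage to an attack window.
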(fn `BeginAttack`)

(fn `EndAttack`)

(fn `GetStateMontageData`
  (params (State :type "/Game/Blueprints/E_CharacterState Enum (by ref)") (Index :type Integer))
  (returns (Montage :type "AnimMontage Object Reference") (Rate :type "Float (double-precision)") (Section :type Name))
  (bind (_montage _rate _section) (`/Game/Blueprints/BFL_GlobalFunctions.FindMontageData` (`self.StateMontageMap`) State Index))
  (return _montage _rate _section))

(fn `ReceiveActorBeginOverlap`
  (params (OtherActor :type "Actor Object Reference"))
  (if (!= OtherActor (`self.GetInstigator`))
    (`GameplayStatics.ApplyDamage` (`local.OtherActor`) (`self.Damage`) (`self.GetInstigatorController`) self)))

(fn `UserConstructionScript`)