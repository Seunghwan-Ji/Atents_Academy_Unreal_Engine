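; Player controller that registers the default Enhanced Input mapping context on BeginPlay and routes player input to the controlled pawn.
; Movement follows control yaw, look drives yaw and pitch, and jump casts the pawn to Character.
; Weapon selection, dodge and begin/end of actions A and B go out as interface-style messages, leaving their behavior to the pawn.
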(event `EnhancedInput|/Game/Input/IA_SelectWeaponA`
  (params (ActionValue :type Boolean) (ElapsedSeconds :type "Float (double-precision)") (TriggeredSeconds :type "Float (double-precision)") (InputAction :type "InputAction Object Reference" :default "/Game/Input/IA_SelectWeaponA.IA_SelectWeaponA"))
  (:`Triggered`
    (message `/Game/Blueprints/BPI_Character.SelectWeaponA` (`self.K2_GetPawn`))))

(event `self.ReceiveBeginPlay`
  (`EnhancedInputSubsystemInterface.AddMappingContext` (subsystem `EnhancedInputLocalPlayerSubsystem`) "/Game/Input/IMC_Default.IMC_Default" 0 (struct)))

(event `EnhancedInput|/Game/Input/IA_SelectWeaponB`
  (params (ActionValue :type Boolean) (ElapsedSeconds :type "Float (double-precision)") (TriggeredSeconds :type "Float (double-precision)") (InputAction :type "InputAction Object Reference" :default "/Game/Input/IA_SelectWeaponB.IA_SelectWeaponB"))
  (:`Triggered`
    (message `/Game/Blueprints/BPI_Character.SelectWeaponB` (`self.K2_GetPawn`))))

(event `EnhancedInput|/Game/Input/IA_Move`
  (params (ActionValue :type "Vector Structure") (ElapsedSeconds :type "Float (double-precision)") (TriggeredSeconds :type "Float (double-precision)") (InputAction :type "InputAction Object Reference" :default "/Game/Input/IA_Move.IA_Move"))
  (bind (_returnvalue_roll _returnvalue_pitch _returnvalue_yaw) (`KismetMathLibrary.BreakRotator` (`self.GetControlRotation`)))
  (bind _returnvalue (`self.K2_GetPawn`))
  (bind _returnvalue_2 (`KismetMathLibrary.MakeRotator` 0.0 0.0 _returnvalue_yaw))
  (:`Triggered`
    (`Pawn.AddMovementInput` _returnvalue (`KismetMathLibrary.GetForwardVector` _returnvalue_2) ActionValue_X false)
    (`Pawn.AddMovementInput` _returnvalue (`KismetMathLibrary.GetRightVector` _returnvalue_2) ActionValue_Y false)))

(event `EnhancedInput|/Game/Input/IA_Look`
  (params (ActionValue :type "Vector2D Structure") (ElapsedSeconds :type "Float (double-precision)") (TriggeredSeconds :type "Float (double-precision)") (InputAction :type "InputAction Object Reference" :default "/Game/Input/IA_Look.IA_Look"))
  (:`Triggered`
    (`self.AddYawInput` ActionValue_X)
    (`self.AddPitchInput` ActionValue_Y)))

(event `EnhancedInput|/Game/Input/IA_Jump`
  (params (ActionValue :type Boolean) (ElapsedSeconds :type "Float (double-precision)") (TriggeredSeconds :type "Float (double-precision)") (InputAction :type "InputAction Object Reference" :default "/Game/Input/IA_Jump.IA_Jump"))
  (bind _returnvalue (`self.K2_GetPawn`))
  (:`Started`
    (bind `_as캐릭터` (cast `Character` _returnvalue))
    (`Character.Jump` `_as캐릭터`))
  (:`Completed`
    (bind `_as캐릭터_2` (cast `Character` _returnvalue))
    (`Character.StopJumping` `_as캐릭터_2`)))

(event `EnhancedInput|/Game/Input/IA_Dodge`
  (params (ActionValue :type Boolean) (ElapsedSeconds :type "Float (double-precision)") (TriggeredSeconds :type "Float (double-precision)") (InputAction :type "InputAction Object Reference" :default "/Game/Input/IA_Dodge.IA_Dodge"))
  (:`Triggered`
    (message `/Game/Blueprints/BPI_Character.Dodge` (`self.K2_GetPawn`))))

(event `EnhancedInput|/Game/Input/IA_ExcuteActionA`
  (params (ActionValue :type Boolean) (ElapsedSeconds :type "Float (double-precision)") (TriggeredSeconds :type "Float (double-precision)") (InputAction :type "InputAction Object Reference" :default "/Game/Input/IA_ExcuteActionA.IA_ExcuteActionA"))
  (bind _returnvalue (`self.K2_GetPawn`))
  (:`Started`
    (message `/Game/Blueprints/BPI_Character.BeginActionA` _returnvalue))
  (:`Completed`
    (message `/Game/Blueprints/BPI_Character.EndActionA` _returnvalue)))

(event `EnhancedInput|/Game/Input/IA_ExcuteActionB`
  (params (ActionValue :type Boolean) (ElapsedSeconds :type "Float (double-precision)") (TriggeredSeconds :type "Float (double-precision)") (InputAction :type "InputAction Object Reference" :default "/Game/Input/IA_ExcuteActionB.IA_ExcuteActionB"))
  (bind _returnvalue (`self.K2_GetPawn`))
  (:`Started`
    (message `/Game/Blueprints/BPI_Character.BeginActionB` _returnvalue))
  (:`Completed`
    (message `/Game/Blueprints/BPI_Character.EndActionB` _returnvalue)))

(fn `UserConstructionScript`)