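; Character Blueprint for dodging, switching between spawned weapons and melee combo attacks, gated by a State variable.
; Weapons start on unequipped sockets; montage notifies move them between sockets, chain swaps, and update movement rotation and the AnimInstance's blend space.
; Attack montages come from the current weapon; anim notify states open combo input windows and start or end hits through BPI_Character.
; Received damage is only printed.
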(event `self.ReceiveBeginPlay`
  (for _array_element (`self.WeaponsClasses`)
    (bind _returnvalue (`|SpawnActorFromClass` _array_element (`/Game/Blueprints/BML_ObjectMacros.DefaultTransform`) "Undefined" "MultiplyWithRoot" self null))
    (`KismetArrayLibrary.Array_Add` (`self.Weapons`) _returnvalue)
    (`self.UnequipWeapon` _returnvalue)))

(event `/Game/Blueprints/BPI_Character.Dodge`
  (bind _returnvalue (`self.GetLastMovementInputVector`))
  (bind _returnvalue_2 (`KismetMathLibrary.Vector_IsZero` _returnvalue))
  (bind _bresult (`self.IsState` "NewEnumerator0"))
  (if _bresult
    (bind _output_get (set `self.State` "NewEnumerator1"))
    (if (not _returnvalue_2)
      (`self.K2_SetActorRotation` (`KismetMathLibrary.MakeRotFromX` _returnvalue)))
    (bind (_montage _rate _section) (`/Game/Blueprints/BFL_GlobalFunctions.FindMontageData` (`self.StateMontageMap`) _output_get (`KismetMathLibrary.Conv_BoolToInt` _returnvalue_2)))
    (`|PlayMontage` (`self.Mesh`) _montage _rate 0.0 _section
      (:`OnBlendOut`
        (set `self.State` "NewEnumerator0")))))

(event `/Game/Blueprints/BPI_Character.BeginActionB`)

(event `/Game/Blueprints/BPI_Character.BeginActionA`
  (bind _bresult (`self.IsArmed`))
  (if _bresult
    (bind _bresult_2 (`self.IsState` "NewEnumerator0"))
    (if _bresult_2
      (bind _output_get (set `self.State` "NewEnumerator3"))
      (bind (_montage _rate _section) (`/Game/Blueprints/BP_Weapon.GetStateMontageData` (`self.CurrentWeapon`) _output_get (`self.AttackIndex`)))
      (`|PlayMontage` (`self.Mesh`) _montage _rate 0.0 _section :!label _label
        (:`OnCompleted`
          (set `self.State` "NewEnumerator0")
          (set `self.AttackIndex` 0))
        (:`OnBlendOut`
          (if (`self.bShouldBeActionTransited`)
            (set `self.bShouldBeActionTransited` false)
            (`/Engine/EditorBlueprintResources/StandardMacros.IncrementInt` (`self.AttackIndex`)
              (:`  `
                (goto _label))))))
      (else
        (bind _bresult_3 (`/Game/Blueprints/BPI_Character.IsState` "NewEnumerator3"))
        (if (and _bresult_3 (`self.bIsInputActionAAllowed`))
          (set `self.bShouldBeActionTransited` true))))))

(event `/Game/Blueprints/BPI_Character.BeginWeaponActionA`
  ; ANS_AttackEnabled 에서 BPI_Character 를 통해 이벤트 호출
  ; 자식(BP_Sword)쪽에서 오버라이드된 함수로 호출
  (`/Game/Blueprints/BP_Weapon.BeginAttack` (`self.CurrentWeapon`)))

(event `/Game/Blueprints/BPI_Character.AllowInputActionA`
  ; ANS_AllowInputActionA 에서 BPI_Character 를 통해 이벤트 호출
  (set `self.bIsInputActionAAllowed` true))

(event `/Game/Blueprints/BPI_Character.DisallowInputActionA`
  ; ANS_AllowInputActionA 에서 BPI_Character 를 통해 이벤트 호출
  (set `self.bIsInputActionAAllowed` false))

(event `/Game/Blueprints/BPI_Character.EndWeaponActionA`
  ; ANS_AttackEnabled 에서 BPI_Character 를 통해 이벤트 호출
  ;; BP_Sword 전달
  ; 자식(BP_Sword)쪽에서 오버라이드된 함수로 호출
  (`/Game/Blueprints/BP_Weapon.EndAttack` (`self.CurrentWeapon`)))

(event `self.ReceiveAnyDamage`
  (params (Damage :type "Float (single-precision)") (DamageType :type "DamageType Object Reference") (InstigatedBy :type "Controller Object Reference") (DamageCauser :type "Actor Object Reference"))
  ; 어떤 주체로부터 Apply Damage 함수를 통해 이 클래스의 객체에게 데미지를 입히려고 할 시 발생하는 이벤트
  (`KismetSystemLibrary.PrintString` (`KismetStringLibrary.Conv_DoubleToString` Damage)))

(event `/Game/Blueprints/BPI_Character.SelectWeaponA`
  (bind _variable (`/Game/Blueprints/BML_ObjectMacros.LocalVariable`))
  (bind _currentweapon (`self.CurrentWeapon`))
  (bind _returnvalue (`SkeletalMeshComponent.GetAnimInstance` (`self.Mesh`)))
  (bind _output (`|GetArrayItem` (`self.Weapons`) _variable))
  (`|VariableSetRef` _variable)
  (bind _bresult (`/Game/Blueprints/BPI_Character.IsState` "NewEnumerator0" :!label _label))
  (if _bresult
    (bind _output_get (set `self.State` "NewEnumerator2"))
    (bind _bresult_2 (`self.IsArmed` :!label _label_2))
    (bind (_montage _rate _section) (`/Game/Blueprints/BP_Weapon.GetStateMontageData` (select `bool` _bresult_2 :`false` _output :`true` (`self.CurrentWeapon`)) _output_get (`KismetMathLibrary.Conv_BoolToInt` _bresult_2)))
    (`|PlayMontage` (`self.Mesh`) _montage _rate 0.0 _section
      (:`OnBlendOut`
        (set `self.State` "NewEnumerator0"))
      (:`OnNotifyBegin`
        (bind _bresult_3 (`self.IsArmed`))
        (if _bresult_3
          (`self.UnequipWeapon` _currentweapon)
          (if (!= _currentweapon _output)
            (set `self.CurrentWeapon` null)
            (goto _label_2)
            (else
              (set `self.CurrentWeapon` null)
              (set `CharacterMovementComponent.bOrientRotationToMovement` true (`self.CharacterMovement`))
              (message `/Game/Blueprints/BPI_CharacterAnimation.SetBSWeapon` _returnvalue null)))
          (else
            (`self.EquipWeapon` _output)
            (bind _output_get_2 (set `self.CurrentWeapon` _output))
            (set `CharacterMovementComponent.bOrientRotationToMovement` false (`self.CharacterMovement`))
            (message `/Game/Blueprints/BPI_CharacterAnimation.SetBSWeapon` _returnvalue (`/Game/Blueprints/BP_Weapon.BlendSpace` _output_get_2))))))))

(event `/Game/Blueprints/BPI_Character.SelectWeaponB`
  (`|VariableSetRef` (`/Game/Blueprints/BML_ObjectMacros.LocalVariable`) 1)
  (goto _label))

(fn `AttachActorToMesh`
  (params (Actor :type "Actor Object Reference") (Socket :type Name))
  (`self.K2_AttachToComponent` Actor (`self.Mesh`) Socket "SnapToTarget" "SnapToTarget" "KeepRelative" true))

(fn `EquipWeapon`
  (params (Weapon :type "/Game/Blueprints/BP_Weapon Object Reference"))
  (`self.AttachActorToMesh` Weapon (`/Game/Blueprints/BP_Weapon.SocketOnEquipped` Weapon)))

(fn `IsArmed`
  (returns (bResult :type Boolean))
  (return (!= null (`self.CurrentWeapon`))))

(fn `IsState`
  (params (State :type "/Game/Blueprints/E_CharacterState Enum" :default "NewEnumerator0"))
  (returns (bResult :type Boolean))
  (return (`|EnumEquality` State (`self.State`))))

(fn `UnequipWeapon`
  (params (Weapon :type "/Game/Blueprints/BP_Weapon Object Reference"))
  (`self.AttachActorToMesh` Weapon (`/Game/Blueprints/BP_Weapon.SocketOnUnequipped` Weapon)))

(fn `UserConstructionScript`)