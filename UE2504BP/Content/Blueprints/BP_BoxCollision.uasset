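; BP_BoxCollision is an actor that demonstrates collision events by printing each one along with the other actor's display name.
; Actor-level begin and end overlap events report overlaps, and the Hit event reports blocking collisions.
; A separate component-level begin overlap is bound only to the Box, so per its comment the child Sphere does not trigger it, contrasting component scope with actor scope.
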(event `self.ReceiveActorBeginOverlap`
  (params (OtherActor :type "Actor Object Reference"))
  ; 다른 충돌체와 오버랩 충돌이 발생했을 때, 충돌이 시작할 때와 끝날 때 발생하는 이벤트
  (`KismetSystemLibrary.PrintString` (`KismetStringLibrary.Concat_StrStr` "ActorBeginOverlap:" (`KismetSystemLibrary.GetDisplayName` OtherActor))))

(event `self.ReceiveActorEndOverlap`
  (params (OtherActor :type "Actor Object Reference"))
  ; 다른 충돌체와 오버랩 충돌이 발생했을 때, 충돌이 시작할 때와 끝날 때 발생하는 이벤트
  (`KismetSystemLibrary.PrintString` (`KismetStringLibrary.Concat_StrStr` "ActorEndOverlap:" (`KismetSystemLibrary.GetDisplayName` OtherActor))))

(event `self.Box.OnComponentBeginOverlap`
  (params (OverlappedComponent :type "PrimitiveComponent Object Reference") (OtherActor :type "Actor Object Reference") (OtherComp :type "PrimitiveComponent Object Reference") (OtherBodyIndex :type Integer) (bFromSweep :type Boolean) (SweepResult :type "HitResult Structure (by ref)"))
  ; Box 전용 오버랩 이벤트, 자식 충돌체인 Sphere 한테는 이 이벤트가 발생하지 않음
  (`KismetSystemLibrary.PrintString` (`KismetStringLibrary.Concat_StrStr` "OnComponentBeginOverlap (Box):" (`KismetSystemLibrary.GetDisplayName` OtherActor))))

(event `self.ReceiveHit`
  (params (MyComp :type "PrimitiveComponent Object Reference") (Other :type "Actor Object Reference") (OtherComp :type "PrimitiveComponent Object Reference") (bSelfMoved :type Boolean) (HitLocation :type "Vector Structure") (HitNormal :type "Vector Structure") (NormalImpulse :type "Vector Structure") (Hit :type "HitResult Structure (by ref)"))
  ; 다른 충돌체와 블록 충돌이 발생했을 때 발생하는 이벤트
  (`KismetSystemLibrary.PrintString` (`KismetStringLibrary.Concat_StrStr` "Hit:" (`KismetSystemLibrary.GetDisplayName` Other))))

(fn `UserConstructionScript`)