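; BP_Sword is a sword weapon Blueprint that adds visual effects while an attack is active.
; It overrides the parent's BeginAttack and EndAttack and calls the parent version first in each.
; BeginAttack starts a weapon trail between the "start" and "end" sockets and activates the Effect component.
; EndAttack ends the trail and deactivates the effect.
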(fn `BeginAttack`
  (`parent.BeginAttack`)
  (`|ExecutionSequence`
    (:`then_0`
      (`ParticleSystemComponent.BeginTrails` (`self.Trail`) "start" "end" "ETrailWidthMode_FromSecond" 1.0))
    (:`then_1`
      (`ActorComponent.Activate` (`self.Effect`) true))))

(fn `EndAttack`
  (`parent.EndAttack`)
  (`|ExecutionSequence`
    (:`then_0`
      (`ParticleSystemComponent.EndTrails` (`self.Trail`)))
    (:`then_1`
      (`ActorComponent.Deactivate` (`self.Effect`)))))

(fn `UserConstructionScript`
  (`parent.UserConstructionScript`))